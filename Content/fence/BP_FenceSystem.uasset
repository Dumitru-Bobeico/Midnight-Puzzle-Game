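; BP_FenceSystem is a procedural fence actor that builds posts and connecting ribbons in its construction script.
; It places a post mesh at each PostTransform point, then adds a raised ribbon mesh aimed at the next point.
; Each ribbon is stretched along X by point distance over its local bounds and given RibbonMat.
; FullLoop links the last post back to the first; the event graph is empty.
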(fn `UserConstructionScript`
  (bind _posttransform (`self.postTransform`))
  (for (_array_element _array_index) _posttransform
    (`AddComponent|NODE_AddStaticMeshComponent-0` :`RelativeTransform` (`KismetMathLibrary.MakeTransform` _array_element))
    (bind _returnvalue (!= _array_index (`KismetArrayLibrary.Array_LastIndex` _posttransform)))
    (if (or _returnvalue (`self.fullLoop?`))
      (bind _output (`|GetArrayItem` _posttransform (`KismetMathLibrary.SelectInt` (+ _array_index 1) 0 _returnvalue)))
      (bind _returnvalue_2 (`AddComponent|NODE_AddStaticMeshComponent-1` :`RelativeTransform` (`KismetMathLibrary.MakeTransform` (+ _array_element (0.0 0.0 90.0)) (`KismetMathLibrary.FindLookAtRotation` _array_element _output))))
      (`SceneComponent.SetRelativeScale3D` _returnvalue_2 (`KismetMathLibrary.MakeVector` (/ (`KismetMathLibrary.Vector_Distance` _array_element _output) (.x (`.Max` (`StaticMeshComponent.GetLocalBounds` _returnvalue_2)))) 1.0 1.0))
      (`PrimitiveComponent.SetMaterial` _returnvalue_2 0 (`self.RibbonMat`)))))