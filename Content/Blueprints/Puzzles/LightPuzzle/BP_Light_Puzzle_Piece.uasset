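; A light puzzle piece Blueprint whose point light changes color each time it is interacted with.
; OnInteract increments ColorIndex, wraps it back to zero past the last color, then calls UpdateLightColor.
; UpdateLightColor switches on the index to set the PointLight to white, green, red or blue.
; It contains no solution check, only the color cycling.
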(event `/Game/Blueprints/Interactables/BPI_Interact.OnInteract`
  (params (Actor :type "Actor Object Reference"))
  (bind _result (`/Engine/EditorBlueprintResources/StandardMacros.IncrementInt` (`self.ColorIndex`))
    (:`  `
      (if (not (<= _result 3))
        (set `self.ColorIndex` 0))
      (`self.UpdateLightColor`))))

(fn `UpdateLightColor`
  (switch `int` (`self.ColorIndex`)
    (:`0`
      (`LightComponent.SetLightColor` (`self.PointLight`) (struct :`R` 1.0 :`G` 1.0 :`B` 1.0 :`A` 1.0) true))
    (:`1`
      (`LightComponent.SetLightColor` (`self.PointLight`) (struct :`R` 0.083954 :`G` 1.0 :`A` 1.0) true))
    (:`2`
      (`LightComponent.SetLightColor` (`self.PointLight`) (struct :`R` 1.0 :`G` 0.025803 :`A` 1.0) true))
    (:`3`
      (`LightComponent.SetLightColor` (`self.PointLight`) (struct :`G` 0.051178 :`B` 1.0 :`A` 1.0) true))))

(fn `UserConstructionScript`)