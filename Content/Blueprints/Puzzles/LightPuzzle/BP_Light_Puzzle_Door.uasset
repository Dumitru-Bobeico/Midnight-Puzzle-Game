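; BP_Light_Puzzle_Door is a light puzzle door that opens when it receives an interact call with a BP_Puzzle_Checker_Button as the actor.
; That call opens a Gate fed by Tick, which then keeps calling Play on a Timeline.
; The Timeline lerps the Cube toward OpenPos by its Alpha, starting from the Cube's current location on each update rather than a stored start position.
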(event `self.ReceiveTick`
  (params (DeltaSeconds :type "Float (single-precision)"))
  (`/Engine/EditorBlueprintResources/StandardMacros.Gate` true :!label _label
    (:`Exit`
      (bind (_direction _alpha) (`Timeline|Timeline`)
        (:`Update`
          (`SceneComponent.K2_SetWorldLocation` (`self.Cube`) (`KismetMathLibrary.VLerp` (`SceneComponent.K2_GetComponentLocation` (`self.Cube`)) (`SceneComponent.K2_GetComponentLocation` (`self.OpenPos`)) _alpha) false false))))))

(event `/Game/Blueprints/Interactables/BPI_Interact.OnInteract`
  (params (Actor :type "Actor Object Reference"))
  (cast `/Game/Blueprints/Puzzles/LightPuzzle/BP_Puzzle_Checker_Button` Actor)
  (goto _label :!via `Open`))

(fn `UserConstructionScript`)