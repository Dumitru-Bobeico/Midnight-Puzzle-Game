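; An interactable puzzle piece for the learning puzzle, identified by its piece number and tinted with its own color.
; On interact it prints its number as a debug string, then passes that number to the referenced puzzle manager, if valid, to update the puzzle message.
; The construction script creates a dynamic instance of the base color material on the static mesh and applies the piece's color.
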(event `/Game/Blueprints/Interactables/BPI_Interact.OnInteract`
  (params (Actor :type "Actor Object Reference"))
  (`KismetSystemLibrary.PrintString` (`KismetStringLibrary.Conv_IntToString` (`self.PuzzlePieceNumber`)))
  (bind _puzzlemanager (`self.PuzzleManager`)
    (:`then`
      (message `/Game/Blueprints/Puzzles/LearningPuzzle/BPI_Puzzle.UpdatePuzzle` _puzzlemanager (`self.PuzzlePieceNumber`)))
    (:`else`)))

(fn `UserConstructionScript`
  (bind _returnvalue (`PrimitiveComponent.CreateDynamicMaterialInstance` (`self.StaticMesh`) 0 "/Game/Blueprints/Puzzles/LearningPuzzle/M_BaseColor.M_BaseColor" "None"))
  (`MaterialInstanceDynamic.SetVectorParameterValue` _returnvalue "BaseColor" (`self.Color`)))