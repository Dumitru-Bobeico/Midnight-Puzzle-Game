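; Manager Blueprint for the Reaction Dots puzzle that lights up buttons at random.
; On BeginPlay it caches every BP_RDButton in the level and starts a looping one-second timer on the Test event.
; Each Test call picks a random button and sets its mesh to the green material, with no reset or input handling here.
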(event `self.ReceiveBeginPlay`
  (bind _outactors (`GameplayStatics.GetAllActorsOfClass` "/Game/Blueprints/Puzzles/ReactionDots/BP_RDButton.BP_RDButton_C"))
  (bind _output_get (set `self.Buttons` _outactors))
  (`KismetSystemLibrary.K2_SetTimer` null "Test" 1.0 true))

(event `Test`
  (`PrimitiveComponent.SetMaterial` (`/Game/Blueprints/Puzzles/ReactionDots/BP_RDButton.StaticMesh` (`|GetArrayItem` (stale `self.ReceiveBeginPlay` _output_get) (`KismetMathLibrary.RandomIntegerInRange` 0 (- (`KismetArrayLibrary.Array_Length` (`self.Buttons`)) 1)))) 0 "/Game/Blueprints/Puzzles/ReactionDots/MAT_RDGreen.MAT_RDGreen"))

(fn `UserConstructionScript`)