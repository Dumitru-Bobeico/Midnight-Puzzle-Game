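; BP_Actor is a physics actor that can rewind its static mesh through its recorded motion.
; While not rewinding, Tick appends the mesh's world transform and velocities to two uncapped arrays.
; Rewind and NotRewind toggle playback, which applies and pops the newest entries each tick, holding the first transform.
; Velocities are packed into transforms, but only linear velocity is restored; the stored angular velocity goes unused.
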(event `/Game/Blueprints/BPI_Rewind.Rewind`
  (set `self.bIsRewinding` true))

(event `/Game/Blueprints/BPI_Rewind.Not Rewind`
  (set `self.bIsRewinding` false))

(event `self.ReceiveTick`
  (params (DeltaSeconds :type "Float (single-precision)"))
  (bind _actorvelocity (`self.ActorVelocity`))
  (bind _actorvelocity_2 (`self.ActorVelocity`))
  (bind _actortransform (`self.ActorTransform`))
  (bind _actortransform_2 (`self.ActorTransform`))
  (bind _actortransform_3 (`self.ActorTransform`))
  (bind _staticmesh (`self.StaticMesh`))
  (bind _returnvalue (`KismetArrayLibrary.Array_LastIndex` _actorvelocity_2))
  (bind _returnvalue_2 (`KismetArrayLibrary.Array_LastIndex` _actortransform_2))
  (bind _output_location (`KismetMathLibrary.BreakTransform` (`|GetArrayItem` _actorvelocity (`KismetArrayLibrary.Array_LastIndex` _actorvelocity))))
  (`|ExecutionSequence`
    (:`then_0`
      (if (`self.bIsRewinding`)
        (if (> (`KismetArrayLibrary.Array_LastIndex` (`self.ActorTransform`)) 0)
          (`SceneComponent.K2_SetWorldTransform` (`self.StaticMesh`) (`|GetArrayItem` _actortransform (`KismetArrayLibrary.Array_LastIndex` _actortransform)) false false)
          (if (> _returnvalue_2 0)
            (`KismetArrayLibrary.Array_Remove` _actortransform_2 _returnvalue_2))
          (else
            (`SceneComponent.K2_SetWorldTransform` (`self.StaticMesh`) (`|GetArrayItem` _actortransform_3 (`KismetArrayLibrary.Array_LastIndex` _actortransform_3)) false false)))
        (else
          (`KismetArrayLibrary.Array_Add` (`self.ActorTransform`) (`SceneComponent.K2_GetComponentToWorld` (`self.StaticMesh`))))))
    (:`then_1`
      (if (`self.bIsRewinding`)
        (if (> (`KismetArrayLibrary.Array_LastIndex` (`self.ActorVelocity`)) 0)
          (`PrimitiveComponent.SetPhysicsLinearVelocity` (`self.StaticMesh`) _output_location false "None")
          (if (> _returnvalue 0)
            (`KismetArrayLibrary.Array_Remove` _actorvelocity_2 _returnvalue)))
        (else
          (bind _returnvalue_3 (`PrimitiveComponent.GetPhysicsLinearVelocity` _staticmesh "None"))
          (`KismetArrayLibrary.Array_Add` (`self.ActorVelocity`) (`KismetMathLibrary.MakeTransform` _returnvalue_3 (struct) (`PrimitiveComponent.GetPhysicsAngularVelocityInDegrees` _staticmesh "None"))))))))

(fn `UserConstructionScript`)