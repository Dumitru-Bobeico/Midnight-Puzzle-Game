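; BP_DoorToNextLevel is an interactable swinging door with a trigger that sends the player to the next level.
; OnInteract alternately plays and reverses a timeline rotating the door's yaw, ignoring input while it animates.
; A dot product of the player's direction and the actor's forward vector picks which way the door swings.
; When the third-person character overlaps the trigger, a fade widget plays before a hardcoded level opens after a short delay.
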(event `self.Trigger.OnComponentBeginOverlap`
  (params (OverlappedComponent :type "PrimitiveComponent Object Reference") (OtherActor :type "Actor Object Reference") (OtherComp :type "PrimitiveComponent Object Reference") (OtherBodyIndex :type Integer) (bFromSweep :type Boolean) (SweepResult :type "HitResult Structure (by ref)"))
  ;[1 1 1] Next Level
  (cast `/Game/ThirdPerson/Blueprints/BP_ThirdPersonCharacter` OtherActor)
  (bind _returnvalue (`|CreateWidget` "/Game/UI/WBP_Fade.WBP_Fade_C"))
  (`UserWidget.AddToViewport` _returnvalue 0)
  (`/Game/UI/WBP_Fade.Fade Anim` _returnvalue)
  (`KismetSystemLibrary.Delay` 1.0)
  (`GameplayStatics.OpenLevel` "1stDoorFinalVerionRemake"))

(event `/Game/Blueprints/Interactables/BPI_Interact.OnInteract`
  (params (Actor :type "Actor Object Reference") (`Player Location` :type "Vector Structure"))
  ;[1 1 1] Door Code
  (if (not (`TimelineComponent.IsPlaying` (`self.DoorTimeline`)))
    (`/Engine/EditorBlueprintResources/StandardMacros.FlipFlop`
      (:`A`
        (`self.SetDoorOpenAngle` `Player Location`)
        (bind (_direction _dooralpha) (`Timeline|DoorTimeline` :!label _label)
          (:`Update`
            (`SceneComponent.K2_SetRelativeRotation` (`self.Door`) (`KismetMathLibrary.MakeRotator` 0.0 0.0 (`KismetMathLibrary.Lerp` 180.0 (`self.DoorOpenAngle`) _dooralpha)) false false))))
      (:`B`
        (goto _label :!via `Reverse`)))))

(fn `SetDoorOpenAngle`
  (params (`Player Location` :type "Vector Structure"))
  ;[1 1 1] Calculate door angle based on the dot product
  (set `self.DoorOpenAngle` (`KismetMathLibrary.SelectFloat` 90.0 270.0 (>= (`KismetMathLibrary.Dot_VectorVector` (`KismetMathLibrary.GetDirectionUnitVector` (`self.K2_GetActorLocation`) (`local.Player Location`)) (`self.GetActorForwardVector`)) 0.0)))
  (return))

(fn `UserConstructionScript`)