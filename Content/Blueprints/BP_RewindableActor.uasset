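; An actor with a physics cube whose motion can be rewound in time through Rewind and StopRewind events.
; Each Tick outside rewind appends the cube's world transform and velocities to two uncapped arrays, packing linear and angular velocity into a transform.
; While rewinding, Tick pops the newest entries to restore transform and linear velocity, holding the oldest transform at the end.
; Angular velocity is recorded but never reapplied.
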(event `/Game/Blueprints/BPI_Rewind.Rewind`
  (set `self.IsRewinding?` true))

(event `/Game/Blueprints/BPI_Rewind.Stop Rewind`
  (set `self.IsRewinding?` false))

(event `self.ReceiveTick`
  (params (DeltaSeconds :type "Float (single-precision)"))
  (bind _cube (`self.Cube`))
  (bind _actorvelocity (`self.ActorVelocity`))
  (bind _actorvelocity_2 (`self.ActorVelocity`))
  (bind _actortransform (`self.ActorTransform`))
  (bind _actortransform_2 (`self.ActorTransform`))
  (bind _actortransform_3 (`self.ActorTransform`))
  (bind _returnvalue (`KismetArrayLibrary.Array_LastIndex` _actorvelocity_2))
  (bind _returnvalue_2 (`KismetArrayLibrary.Array_LastIndex` _actortransform_2))
  (bind _output_location (`KismetMathLibrary.BreakTransform` (`|GetArrayItem` _actorvelocity (`KismetArrayLibrary.Array_LastIndex` _actorvelocity))))
  (`|ExecutionSequence`
    (:`then_0`
      (if (`self.IsRewinding?`)
        (if (> (`KismetArrayLibrary.Array_LastIndex` (`self.ActorTransform`)) 0)
          (`SceneComponent.K2_SetWorldTransform` (`self.Cube`) (`|GetArrayItem` _actortransform (`KismetArrayLibrary.Array_LastIndex` _actortransform)) false false)
          (if (> _returnvalue_2 0)
            (`KismetArrayLibrary.Array_Remove` _actortransform_2 _returnvalue_2))
          (else
            (`SceneComponent.K2_SetWorldTransform` (`self.Cube`) (`|GetArrayItem` _actortransform_3 (`KismetArrayLibrary.Array_LastIndex` _actortransform_3)) false false)))
        (else
          (`KismetArrayLibrary.Array_Add` (`self.ActorTransform`) (`SceneComponent.K2_GetComponentToWorld` (`self.Cube`))))))
    (:`then_1`
      (if (`self.IsRewinding?`)
        (if (> (`KismetArrayLibrary.Array_LastIndex` (`self.ActorVelocity`)) 0)
          (`PrimitiveComponent.SetPhysicsLinearVelocity` (`self.Cube`) _output_location false "None")
          (if (> _returnvalue 0)
            (`KismetArrayLibrary.Array_Remove` _actorvelocity_2 _returnvalue)))
        (else
          (bind _returnvalue_3 (`PrimitiveComponent.GetPhysicsLinearVelocity` _cube "None"))
          (`KismetArrayLibrary.Array_Add` (`self.ActorVelocity`) (`KismetMathLibrary.MakeTransform` _returnvalue_3 (struct) (`PrimitiveComponent.GetPhysicsAngularVelocityInDegrees` _cube "None"))))))))

(fn `UserConstructionScript`)