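; Hinged door Blueprint that swings DoorMesh open and closed.
; BeginPlay caches the mesh's relative rotation as the closed pose, and a timeline lerps from it to the OpenPos component's rotation.
; OpenDoor plays the timeline and CloseDoor reverses it, each updating IsOpen.
; The construction script calls its parent, then snaps the mesh to the open rotation when IsOpen is set.
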(event `self.ReceiveBeginPlay`
  (set `self.Default Relative Rotation` (`SceneComponent.RelativeRotation` (`self.DoorMesh`))))

(event `self.OpenDoor`
  (params (ThirdPersonActor :type "/Game/ThirdPerson/Blueprints/BP_ThirdPersonCharacter Object Reference"))
  (set `self.isOpen?` true)
  (bind (_direction _alpha) (`Timeline|DoorMove_Timeline` :!label _label)
    (:`Update`
      (`SceneComponent.K2_SetRelativeRotation` (`self.DoorMesh`) (`KismetMathLibrary.RLerp` (`self.Default Relative Rotation`) (`SceneComponent.RelativeRotation` (`self.OpenPos`)) _alpha) false false))))

(event `self.CloseDoor`
  (params (ThirdPersonActor :type "/Game/ThirdPerson/Blueprints/BP_ThirdPersonCharacter Object Reference"))
  (set `self.isOpen?` false)
  (goto _label :!via `Reverse`))

(fn `UserConstructionScript`
  (`parent.UserConstructionScript`)
  (if (`self.isOpen?`)
    (`SceneComponent.K2_SetRelativeRotation` (`self.DoorMesh`) (`SceneComponent.RelativeRotation` (`self.OpenPos`)) false false)))