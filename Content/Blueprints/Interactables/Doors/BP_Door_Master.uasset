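; BP_Door_Master is a base door Blueprint that players toggle through a Door interact event.
; An open door closes, and a closed door opens unless it is locked.
; Locked doors open only if the interacting character has the KeyItem, otherwise a debug message prints in place of a planned locked sound.
; OpenDoor and CloseDoor are empty events here, with no movement logic in this file.
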(event `/Game/Blueprints/Interactables/BPI_Interact.Interact(Door)`
  (params (ThirdPersonActor :type "/Game/ThirdPerson/Blueprints/BP_ThirdPersonCharacter Object Reference"))
  (if (`self.isOpen?`)
    (`self.CloseDoor` null)
    (elif (`self.isLocked?`)
      (bind _result (`/Game/ThirdPerson/Blueprints/BP_ThirdPersonCharacter.CheckHasItem` ThirdPersonActor (`self.KeyItem`)))
      (if _result
        (`self.OpenDoor` ThirdPersonActor)
        (else
          (`KismetSystemLibrary.PrintString` "Door Is Locked (Throw a sound to show its locked)")))
      (else
        (`self.OpenDoor` ThirdPersonActor)))))

(event `CloseDoor`
  (params (ThirdPersonActor :type "/Game/ThirdPerson/Blueprints/BP_ThirdPersonCharacter Object Reference")))

(event `OpenDoor`
  (params (ThirdPersonActor :type "/Game/ThirdPerson/Blueprints/BP_ThirdPersonCharacter Object Reference")))

(fn `UserConstructionScript`)