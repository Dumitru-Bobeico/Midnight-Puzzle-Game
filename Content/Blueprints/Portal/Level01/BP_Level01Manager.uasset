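; Level 1 manager for a portal puzzle that swaps which right and wrong portals are visible and collidable as the player makes choices.
; Later-stage portals start hidden, and entering the wrong portal swaps the first right portal for the second.
; Each exit from the entrance portal increments a counter; once it reaches a threshold after a wrong pick, the third pair replaces the current portals.
; Entering the right portal only sets a flag.
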(event `self.ReceiveBeginPlay`
  (bind _portalright2 (`self.PortalRight2`))
  (bind _portalwrong3 (`self.PortalWrong3`))
  (bind _portalright3 (`self.PortalRight3`))
  (`self.SetActorHiddenInGame` _portalright2 true)
  (`self.SetActorEnableCollision` _portalright2 false)
  (`self.SetActorHiddenInGame` _portalright3 true)
  (`self.SetActorEnableCollision` _portalright3 false)
  (`self.SetActorHiddenInGame` _portalwrong3 true)
  (`self.SetActorEnableCollision` _portalwrong3 false))

(event `self.PortalWrong.OnActorBeginOverlap`
  (params (OverlappedActor :type "Actor Object Reference") (OtherActor :type "Actor Object Reference"))
  (bind _portalright (`self.PortalRight`))
  (bind _portalright2 (`self.PortalRight2`))
  (set `self.PickedWrong` true)
  (`self.SetActorHiddenInGame` _portalright true)
  (`self.SetActorEnableCollision` _portalright false)
  (`self.SetActorHiddenInGame` _portalright2 false)
  (`self.SetActorEnableCollision` _portalright2 true))

(event `self.PortalRight.OnActorBeginOverlap`
  (params (OverlappedActor :type "Actor Object Reference") (OtherActor :type "Actor Object Reference"))
  (set `self.PickedRight` true))

(event `self.EntrancePortal.OnActorEndOverlap`
  (params (OverlappedActor :type "Actor Object Reference") (OtherActor :type "Actor Object Reference"))
  (bind _portalright2 (`self.PortalRight2`))
  (bind _portalwrong (`self.PortalWrong`))
  (bind _portalwrong3 (`self.PortalWrong3`))
  (bind _portalright3 (`self.PortalRight3`))
  (bind _result (`/Engine/EditorBlueprintResources/StandardMacros.IncrementInt` (`self.CounterWrong`))
    (:`  `
      (set `self.CounterWrong` _result)
      (`KismetSystemLibrary.PrintString` (`KismetStringLibrary.Conv_IntToString` (`self.CounterWrong`)))
      (`KismetSystemLibrary.PrintString` (`KismetStringLibrary.Conv_BoolToString` (`self.PickedWrong`)))
      (if (`self.PickedWrong`)
        (bind _output_get (set `self.PickedWrong2` true))
        (if _output_get
          (if (>= (`self.CounterWrong`) 3)
            (`self.SetActorHiddenInGame` _portalwrong true)
            (`self.SetActorEnableCollision` _portalwrong false)
            (`self.SetActorHiddenInGame` _portalwrong3 false)
            (`self.SetActorEnableCollision` _portalwrong3 true)
            (`self.SetActorHiddenInGame` _portalright2 true)
            (`self.SetActorEnableCollision` _portalright2 false)
            (`self.SetActorHiddenInGame` _portalright3 false)
            (`self.SetActorEnableCollision` _portalright3 true)))))))

(fn `UserConstructionScript`)