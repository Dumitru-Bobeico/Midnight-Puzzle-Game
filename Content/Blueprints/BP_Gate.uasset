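; BP_Gate is a double-door gate that opens and closes automatically from BeginPlay.
; Move uses a FlipFlop to alternate playing and reversing MoveTimeline, whose alpha lerps each door between its start and end marker locations.
; When the timeline finishes, it plays a quiet explosion sound at the left start marker, waits briefly and calls Move again to continue the cycle.
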(event `self.ReceiveBeginPlay`
  (`self.Move`))

(event `Move`
  (`/Engine/EditorBlueprintResources/StandardMacros.FlipFlop`
    (:`A`
      (bind (_direction _alpha) (`Timeline|MoveTimeline` :!label _label)
        (:`Update`
          (`SceneComponent.K2_SetRelativeLocation` (`self.leftDoor`) (`KismetMathLibrary.VLerp` (`SceneComponent.RelativeLocation` (`self.left_startLoc`)) (`SceneComponent.RelativeLocation` (`self.left_endLoc`)) _alpha) false false)
          (`SceneComponent.K2_SetRelativeLocation` (`self.rightDoor`) (`KismetMathLibrary.VLerp` (`SceneComponent.RelativeLocation` (`self.right_startLoc`)) (`SceneComponent.RelativeLocation` (`self.right_endLoc`)) _alpha) false false))
        (:`Finished`
          (`GameplayStatics.PlaySoundAtLocation` "/Game/StarterContent/Audio/Explosion02.Explosion02" (`SceneComponent.K2_GetComponentLocation` (`self.left_startLoc`)) (struct) 0.1 1.0 0.0 null null null null)
          (`KismetSystemLibrary.Delay` 1.0)
          (`self.Move`))))
    (:`B`
      (goto _label :!via `Reverse`))))

(fn `UserConstructionScript`)